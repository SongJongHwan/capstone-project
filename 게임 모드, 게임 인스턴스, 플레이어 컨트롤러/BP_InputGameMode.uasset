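; BP_InputGameMode is a game mode that sets up the on-screen widget and carries player stats in from the game instance.
; On BeginPlay it adds NewWidgetBlueprint to the viewport and copies Health, Bomb and Portion from level_item into player_V2.
; Tick polls player health; while it is zero or below, it removes the widget and resets the stored Portion and Bomb to fixed defaults, leaving stored Health untouched.
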(event `self.ReceiveBeginPlay`
  (bind _returnvalue (`|CreateWidget` "/Game/자료/UI/NewWidgetBlueprint.NewWidgetBlueprint_C"))
  (`UserWidget.AddToViewport` _returnvalue 0)
  (bind _asplayer_v2 (cast `/Game/자료/플레이어/player_V2` (`GameplayStatics.GetPlayerCharacter` 0)))
  (bind _aslevel_item (cast `/Game/Blueprints/level_item` (`GameplayStatics.GetGameInstance`)))
  (bind _health (`/Game/Blueprints/level_item.Get Health` _aslevel_item))
  (set `/Game/자료/플레이어/player_V2.Health` _health _asplayer_v2)
  (bind _bomb (`/Game/Blueprints/level_item.Get bomb` _aslevel_item))
  (set `/Game/자료/플레이어/player_V2.bomb` _bomb _asplayer_v2)
  (bind _portion (`/Game/Blueprints/level_item.Get portion` _aslevel_item))
  (set `/Game/자료/플레이어/player_V2.portion` _portion _asplayer_v2))

(event `self.ReceiveTick`
  (params (DeltaSeconds :type "Float (single-precision)"))
  (bind _asplayer_v2 (cast `/Game/자료/플레이어/player_V2` (`GameplayStatics.GetPlayerCharacter` 0)))
  (if (<= (`/Game/자료/플레이어/player_V2.Health` _asplayer_v2) 0.0)
    (`Widget.RemoveFromParent` (stale `self.ReceiveBeginPlay` _returnvalue))
    (bind _aslevel_item (cast `/Game/Blueprints/level_item` (`GameplayStatics.GetGameInstance`)))
    (`/Game/Blueprints/level_item.Set Portion` _aslevel_item 1)
    (`/Game/Blueprints/level_item.Set Bomb` _aslevel_item 3)))

(fn `UserConstructionScript`)